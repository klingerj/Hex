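; Hex grid tile actor that shows a movement path under the cursor and acts as a clickable move target.
; Hovering has HexGridGraphManagerBP trace the shortest path backwards from the tile; leaving resets it.
; Tick recolors tiles through newly created dynamic materials: grey off-path, green-to-red by DistanceToMove on-path during GameManagerBP stage 3.
; Clicking in that stage sets the turn player's tile if DistanceToMove is at most 2.
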(event `self.ReceiveActorEndCursorOver`
  (bind _tilemesh (`self.TileMesh`))
  (bind _tilemesh_2 (`self.TileMesh`))
  (bind _output (`|GetArrayItem` (stale `self.ReceiveActorBeginCursorOver` _outactors)))
  (`/Engine/EditorBlueprintResources/StandardMacros.IsValid` _output
    (:`Is Valid`
      (bind _output_2 (`|GetArrayItem` (stale `self.ReceiveActorEndCursorOver` _outactors)))
      (`/Engine/EditorBlueprintResources/StandardMacros.IsValid` _output_2
        (:`Is Valid`
          (`HexGridGraphManager.ResetShortestPath` _output)
          (if (`self.onShortestPath`) :!label _label
            (bind _outactors (`GameplayStatics.GetAllActorsOfClass` "/Game/Blueprints/GameManagerBP.GameManagerBP_C" :!label _label_2))
            (if (> (`KismetArrayLibrary.Array_Length` _outactors) 0)
              (`/Engine/EditorBlueprintResources/StandardMacros.IsValid` _output_2
                (:`Is Valid`
                  (if (and (`self.onShortestPath`) (== (`GameManager.GetStage` _output_2) 3))
                    (bind _returnvalue (`PrimitiveComponent.CreateDynamicMaterialInstance` _tilemesh_2 0 (`PrimitiveComponent.GetMaterial` _tilemesh_2 0) "None"))
                    (`MaterialInstanceDynamic.SetVectorParameterValue` _returnvalue (`KismetStringLibrary.Conv_StringToName` "BaseColor") (`KismetMathLibrary.LinearColorLerp` (make `LinearColor` 0.0 1.0) (make `LinearColor` 1.0) (/ (`KismetMathLibrary.Conv_IntToDouble` (`self.distanceToMove`)) 3.0)))))))
            (else
              (bind _returnvalue_2 (`PrimitiveComponent.CreateDynamicMaterialInstance` _tilemesh 0 (`PrimitiveComponent.GetMaterial` _tilemesh 0) "None"))
              (`MaterialInstanceDynamic.SetVectorParameterValue` _returnvalue_2 (`KismetStringLibrary.Conv_StringToName` "BaseColor") (make `LinearColor` 0.2 0.2 0.2 1.0)))))))))

(event `self.ReceiveTick`
  (params (DeltaSeconds :type "Float (single-precision)"))
  (goto _label))

(event `self.ReceiveActorBeginCursorOver`
  (bind _outactors (`GameplayStatics.GetAllActorsOfClass` "/Game/Blueprints/HexGridGraphManagerBP.HexGridGraphManagerBP_C"))
  (if (> (`KismetArrayLibrary.Array_Length` _outactors) 0)
    (bind _output (`|GetArrayItem` _outactors))
    (`/Engine/EditorBlueprintResources/StandardMacros.IsValid` _output
      (:`Is Valid`
        (`HexGridGraphManager.ResetShortestPath` _output)
        (`HexGridGraphManager.SetShortestPath_Backwards` _output self)
        (goto _label_2)))))

(event `self.ReceiveActorOnClicked`
  (params (ButtonPressed :type "Key Structure"))
  (if (> (`KismetArrayLibrary.Array_Length` (stale `self.ReceiveActorEndCursorOver` _outactors)) 0)
    (bind _output (`|GetArrayItem` (stale `self.ReceiveActorEndCursorOver` _outactors)))
    (`/Engine/EditorBlueprintResources/StandardMacros.IsValid` _output
      (:`Is Valid`
        (if (and (== (`GameManager.GetStage` _output) 3) (<= (`self.distanceToMove`) 2))
          (`GameManager.SetTurnPlayerTile` _output self)
          (`HexGridGraphManager.ResetShortestPath` (`|GetArrayItem` (stale `self.ReceiveActorBeginCursorOver` _outactors))))))))

(fn `UserConstructionScript`)