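; Floating resource pickup visual for a hex grid tile, bobbing on a clock-driven sine wave.
; Every Tick it sets mesh by Type, recreates a rarity-tinted dynamic material, and searches all tiles for TileID.
; It hides during tile cooldown, firing YellResource at four turns remaining, with GameManagerBP's SuckOnThis blocking immediate repeats since PrevIsOnCD is never set true.
; Cursor overlap events update the manager's hovered object.
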(event `self.ReceiveTick`
  (params (DeltaSeconds :type "Float (single-precision)"))
  (bind _returnvalue (`KismetStringLibrary.Conv_StringToName` "BaseColor"))
  (bind _returnvalue_2 (`KismetMathLibrary.UtcNow`))
  (bind _linearcolor (make `LinearColor` 0.3 0.85 0.3 0.2))
  (bind _mesh (`self.Mesh`))
  (bind _mesh_2 (`self.Mesh`))
  (`self.K2_SetActorTransform` (`KismetMathLibrary.MakeTransform` (`KismetMathLibrary.MakeVector` (.x (`self.K2_GetActorLocation`)) (.y (`self.K2_GetActorLocation`)) (+ (* (`KismetMathLibrary.Sin` (* (+ (`KismetMathLibrary.Conv_IntToDouble` (`KismetMathLibrary.GetMillisecond` _returnvalue_2)) (* (`KismetMathLibrary.Conv_IntToDouble` (`KismetMathLibrary.GetSecond` _returnvalue_2)) 1000.0)) 0.0006)) 8.0) 30.0))))
  (switch `int` (`self.type`)
    (:`0`
      _)
    (:`1`
      (`StaticMeshComponent.SetStaticMesh` _mesh_2 "/Game/Assets/Models/FatGem.FatGem")))
  (`PrimitiveComponent.CreateDynamicMaterialInstance` _mesh_2 0 (`PrimitiveComponent.GetMaterial` _mesh_2 0) "None")
  (switch `int` (`self.rarity`)
    (:`0`
      (`MeshComponent.SetVectorParameterValueOnMaterials` _mesh _returnvalue (`KismetMathLibrary.Conv_LinearColorToVector` (make `LinearColor` 1.0 0.6 0.8 0.2))))
    (:`1`
      (`MeshComponent.SetVectorParameterValueOnMaterials` _mesh _returnvalue (`KismetMathLibrary.Conv_LinearColorToVector` _linearcolor)))
    (:`2`
      (`MeshComponent.SetVectorParameterValueOnMaterials` _mesh _returnvalue (`KismetMathLibrary.Conv_LinearColorToVector` _linearcolor)))
    (:`3`
      (`MeshComponent.SetVectorParameterValueOnMaterials` _mesh _returnvalue (`KismetMathLibrary.Conv_LinearColorToVector` (make `LinearColor` 0.8 0.65 0.1 1.0)))))
  (bind _outactors (`GameplayStatics.GetAllActorsOfClass` "/Game/Blueprints/HexGridTileBP.HexGridTileBP_C"))
  (for (_array_element _array_index) _outactors
    (if (== (`/Game/Blueprints/HexGridTileBP.ID` _array_element) (`self.TileID`))
      (break)))
  (bind _output (`|GetArrayItem` _outactors _array_index))
  (bind _output_2 (`|GetArrayItem` (`self.K2_GetComponentsByClass` _output "/Script/Hex.HexGridTileEffect")))
  (if (`HexGridTileEffect.IsOnCooldown` _output_2)
    (`self.SetActorHiddenInGame` true)
    (bind _returnvalue_3 (and (== (`HexGridTileEffect.remainingCooldownTurns` _output_2) 4) (not (`self.prevIsOnCD`))))
    (if _returnvalue_3
      (set `self.prevIsOnCD` false)
      (bind _outactors_2 (`GameplayStatics.GetAllActorsOfClass` "/Game/Blueprints/GameManagerBP.GameManagerBP_C"))
      (bind _output_3 (`|GetArrayItem` _outactors_2))
      (`/Engine/EditorBlueprintResources/StandardMacros.IsValid` _output_3
        (:`Is Valid`
          (if (!= self (`/Game/Blueprints/GameManagerBP.SuckOnThis` _output_3))
            (`self.YellResource` (`self.type`) (`self.rarity`) (`HexGridTile.element` _output))
            (set `/Game/Blueprints/GameManagerBP.SuckOnThis` self _output_3 :!label _label)))
        (:`Is Not Valid`
          (goto _label))))
    (else
      (`self.SetActorHiddenInGame` false)
      (if _returnvalue_3
        _))))

(event `self.ReceiveActorBeginCursorOver`
  (if (not (`self.bHidden`))
    (bind _outactors (`GameplayStatics.GetAllActorsOfClass` "/Game/Blueprints/GameManagerBP.GameManagerBP_C"))
    (set `/Game/Blueprints/GameManagerBP.CurrentlyHoveredOverThing` self (`|GetArrayItem` _outactors))))

(event `self.ReceiveActorEndCursorOver`
  (bind _outactors (`GameplayStatics.GetAllActorsOfClass` "/Game/Blueprints/GameManagerBP.GameManagerBP_C"))
  (bind _output (`|GetArrayItem` _outactors))
  (if (== self (`/Game/Blueprints/GameManagerBP.CurrentlyHoveredOverThing` _output))
    (set `/Game/Blueprints/GameManagerBP.CurrentlyHoveredOverThing` null _output)))

(fn `UserConstructionScript`)