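; Hex grid generator actor that spawns a square GridDim-by-GridDim field of HexGridTileBP tiles from its own location on BeginPlay.
; It spawns the origin tile first, then uses that tile's mesh scale, with Y and Z swapped, to space the rest.
; Odd rows are offset half a step, and each tile receives its row/column index via SetGridIndex.
; It also enables the mouse cursor and mouse-over events.
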(event `self.ReceiveBeginPlay`
  (bind _returnvalue (`self.K2_GetActorLocation`))
  (bind _returnvalue_2 (`GameplayStatics.GetPlayerController` 0))
  (bind _returnvalue_3 (- (`self.gridDim`) 1))
  (set `PlayerController.bShowMouseCursor` true _returnvalue_2)
  (set `PlayerController.bEnableMouseOverEvents` true _returnvalue_2)
  (`|SpawnActorFromClass` "/Game/Blueprints/HexGridTileBP.HexGridTileBP_C" (`KismetMathLibrary.Conv_VectorToTransform` _returnvalue) "AlwaysSpawn" "OverrideRootScale" null null)
  (bind _outactors (`GameplayStatics.GetAllActorsOfClass` "/Game/Blueprints/HexGridTileBP.HexGridTileBP_C"))
  (bind _output (`|GetArrayItem` _outactors))
  (set `/Game/Blueprints/HexGridTileBP.gridIndexX` 0 _output)
  (set `/Game/Blueprints/HexGridTileBP.gridIndexY` 0 _output)
  (`HexGridTile.SetGridIndex` _output)
  (for _index (range (+ _returnvalue_3 1))
    (for _index_2 (range (`KismetMathLibrary.Conv_BoolToInt` (== _index 0)) (+ _returnvalue_3 1))
      (bind _returnvalue_4 (`KismetMathLibrary.Conv_IntToDouble` _index))
      (bind _returnvalue_5 (`|SpawnActorFromClass` "/Game/Blueprints/HexGridTileBP.HexGridTileBP_C" (`KismetMathLibrary.MakeTransform` (+ (* (`KismetMathLibrary.MakeVector` (+ (* (`KismetMathLibrary.Conv_IntToDouble` _index_2) 2.0) (* (mod _returnvalue_4 2.0) 1.0)) (* _returnvalue_4 1.75)) (`KismetMathLibrary.MakeVector` (.x (`SceneComponent.K2_GetComponentScale` (`/Game/Blueprints/HexGridTileBP.TileMesh` _output))) (.z (`SceneComponent.K2_GetComponentScale` (`/Game/Blueprints/HexGridTileBP.TileMesh` _output))) (.y (`SceneComponent.K2_GetComponentScale` (`/Game/Blueprints/HexGridTileBP.TileMesh` _output))))) _returnvalue)) "AlwaysSpawn" "OverrideRootScale" null null))
      (set `/Game/Blueprints/HexGridTileBP.gridIndexX` _index _returnvalue_5)
      (set `/Game/Blueprints/HexGridTileBP.gridIndexY` _index_2 _returnvalue_5)
      (`HexGridTile.SetGridIndex` _returnvalue_5))))

(fn `UserConstructionScript`)